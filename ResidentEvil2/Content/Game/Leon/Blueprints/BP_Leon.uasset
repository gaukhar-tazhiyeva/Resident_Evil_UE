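; BP_Leon is the player character, with Enhanced Input movement, camera rotation, sprinting and an over-the-shoulder style aim mode.
; Yaw turns the controller while clamped pitch rotates the spring arm directly.
; Aiming shows WBP_Aim, stops orient-to-movement and plays a timeline that blends spring arm length and socket offset, reversing on release.
; Sprint toggles walk speed; the aim timeline slows it on every update, including the reverse.
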(event Input|EnhancedActionEvents|EnhancedInputActionIA_RotateCamera
  (params (ActionValue :type Vector%202D%20Structure) (ElapsedSeconds :type Float%20%28double-precision%29) (TriggeredSeconds :type Float%20%28double-precision%29) (InputAction :type Input%20Action%20Object%20Reference :default "/Game/Game/Leon/Input/IA_RotateCamera.IA_RotateCamera"))
  (bind (_x _y) (Math|Vector2D|BreakVector2D ActionValue))
  (Pawn|Input|AddControllerYawInput _x)
  (Variables|Default|SetV%20Angle (Math|Float|ClampAngle (+ _y (Variables|Default|GetV%20Angle)) -6e+01 45.0))
  (Transformation|SetRelativeRotation (Variables|Default|GetSpringArm) (Math|Rotator|MakeRotator 0.0 (Variables|Default|GetV%20Angle) (.yaw (Variables|/Script/Engine.SceneComponent|GetRelativeRotation (Variables|Default|GetSpringArm)))) false false))

(event Input|EnhancedActionEvents|EnhancedInputActionIA_Move
  (params (ActionValue :type Vector%202D%20Structure) (ElapsedSeconds :type Float%20%28double-precision%29) (TriggeredSeconds :type Float%20%28double-precision%29) (InputAction :type Input%20Action%20Object%20Reference :default "/Game/Game/Leon/Input/IA_Move.IA_Move"))
  (bind _returnvalue (Pawn|GetControlRotation :!class /Script/Engine.Pawn))
  (bind (_x _y) (Math|Vector2D|BreakVector2D ActionValue))
  (Pawn|Input|AddMovementInput (+ (* _x (Math|Vector|GetForwardVector _returnvalue)) (* _y (Math|Vector|GetRightVector _returnvalue))) 1.0 false))

(event Input|EnhancedActionEvents|EnhancedInputActionIA_Aim
  (params (ActionValue :type Boolean) (ElapsedSeconds :type Float%20%28double-precision%29) (TriggeredSeconds :type Float%20%28double-precision%29) (InputAction :type Input%20Action%20Object%20Reference :default "/Game/Game/Leon/Input/IA_Aim.IA_Aim"))
  (bind _springarm (Variables|Default|GetSpringArm))
  (:Started
    (bind _returnvalue (UserInterface|CreateWidget "/Game/Game/Leon/UI/WBP_Aim.WBP_Aim_C"))
    (UserInterface|Viewport|AddtoViewport _returnvalue 0)
    (bind _newtrack_0 (Timeline|Aim%20Timeline Play)
      (:Update
        (Variables|/Script/Engine.SpringArmComponent|SetTargetArmLength _springarm (Math|Float|Lerp (Variables|Default|GetFree%20Mode%20Target%20Offset) (Variables|Default|GetAim%20Mode%20Target%20Offset) _newtrack_0))
        (Variables|/Script/Engine.SpringArmComponent|SetSocketOffset _springarm (Math|Vector|Lerp(Vector) (Variables|Default|GetFree%20Mode%20Socket%20Offset) (Variables|Default|GetAim%20Mode%20Socket%20Offset) _newtrack_0))
        (Variables|/Script/Engine.CharacterMovementComponent|SetMaxWalkSpeed (Variables|Character|GetCharacterMovement) 5e+01))))
  (:Ongoing
    (Variables|/Script/Engine.CharacterMovementComponent|SetbOrientRotationToMovement (Variables|Character|GetCharacterMovement) false))
  (:Completed
    (Widget|RemovefromParent _returnvalue)
    (Variables|/Script/Engine.CharacterMovementComponent|SetbOrientRotationToMovement (Variables|Character|GetCharacterMovement) true)
    (Timeline|Aim%20Timeline Reverse)))

(event Input|EnhancedActionEvents|EnhancedInputActionIA_Sprint
  (params (ActionValue :type Boolean) (ElapsedSeconds :type Float%20%28double-precision%29) (TriggeredSeconds :type Float%20%28double-precision%29) (InputAction :type Input%20Action%20Object%20Reference :default "/Game/Game/Leon/Input/IA_Sprint.IA_Sprint"))
  (:Started
    (Variables|/Script/Engine.CharacterMovementComponent|SetMaxWalkSpeed (Variables|Character|GetCharacterMovement) 5e+02))
  (:Completed
    (Variables|/Script/Engine.CharacterMovementComponent|SetMaxWalkSpeed (Variables|Character|GetCharacterMovement) 1.5e+02)))

(event EventBeginPlay
  (Input|AddMappingContext (PlayerController|LocalPlayerSubsystems|GetEnhancedInputLocalPlayerSubsystem (Game|GetPlayerController 0)) "/Game/Game/Leon/Input/IMC_Leon.IMC_Leon" 0 "(bIgnoreAllPressedKeysUntilRelease=True,bForceImmediately=False,bNotifyUserSettings=False)"))

(fn ConstructionScript)