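; Shotgun weapon Blueprint that overrides fire effects, reload sound and hit detection, and creates its own crosshair widget on BeginPlay.
; LineTrace fires multiple pellet traces from Leon's camera, each randomly spread within a cone around the view direction.
; Each trace applies damage, boosted for Head bone hits, and spawns a metal impact emitter, with persistent debug lines and bone-name printing left on.
; PlayFX handles fire sound, muzzle flash and camera shake.
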(event EventBeginPlay
  (|CallParentFunction)
  (bind _returnvalue (UserInterface|CreateWidget "/Game/Game/Weapons/UI_Shotgun.UI_Shotgun_C"))
  (Variables|Default|SetCrosshair%20UI _returnvalue))

(fn ConstructionScript
  (|CallParentFunction))

(fn PlayFX
  (Audio|PlaySound2D "/Game/MilitaryWeapDark/Sound/Shotgun/ShotgunB_Fire_Cue.ShotgunB_Fire_Cue" 1.0 1.0 0.0 0 0)
  (Components|Activation|Activate (Variables|Default|GetFlashFX) true)
  (Camera|PlayWorldCameraShake "/Game/Game/Weapons/CS_Shotgun.CS_Shotgun_C" (.location (Default|GetCamTransform (Variables|Default|GetLeon%20Ref))) 0.0 1e+02))

(fn Reload
  (Audio|PlaySound2D "/Game/MilitaryWeapDark/Sound/Shotgun/Wavs/Shotgun_Reload03.Shotgun_Reload03" 1.0 1.0 0.0 0 0))

(fn LineTrace
  (bind (_start _end) (CallFunction|GetLInetraceParams))
  (bind _weapon_damage (Variables|Default|GetWeapon%20Damage))
  (for _index (range 0 7)
    (bind _outhit (Collision|LineTraceByChannel _start _end "TraceTypeQuery1" false (Utilities|Array|MakeArray (Variables|Default|GetLeon%20Ref)) "Persistent"))
    (Utilities|FlowControl|Sequence
      (:then_0
        (Game|Damage|ApplyDamage (.HitActor (Collision|BreakHitResult _outhit)) (Math|Float|SelectFloat (* _weapon_damage 1.5) _weapon_damage (== (.HitBoneName (Collision|BreakHitResult _outhit)) "Head")) 0 0)
        (Development|PrintString (Utilities|String|ToString(Name) (.HitBoneName (Collision|BreakHitResult _outhit)))))
      (:then_1
        (Effects|SpawnEmitteratLocation "/Game/MilitaryWeapDark/FX/P_Impact_Metal_Medium_01.P_Impact_Metal_Medium_01" (.ImpactPoint (Collision|BreakHitResult _outhit)) (Math|Rotator|MakeRotfromX (.ImpactNormal (Collision|BreakHitResult _outhit))))))))

(fn GetLInetraceParams
  (bind _leon_ref (Variables|Default|GetLeon%20Ref))
  (bind _cone_half_angle_in_degrees (Variables|Default|GetCone%20Half%20Angle%20in%20Degrees))
  (bind _cam_transform (Default|GetCamTransform _leon_ref))
  (bind _returnvalue (Math|Vector|GetForwardVector (.rotation _cam_transform)))
  (bind _returnvalue_2 (Math|Random|RandomUnitVectorinConeinDegrees _returnvalue _cone_half_angle_in_degrees))
  (return (.location _cam_transform) (+ (+ (.location _cam_transform) (* _returnvalue_2 1e+03)) _returnvalue_2)))