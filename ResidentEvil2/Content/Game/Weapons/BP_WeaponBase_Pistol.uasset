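; Pistol weapon Blueprint that provides hitscan shooting, fire effects and a reload sound for the character held in LeonRef.
; LineTrace fires a Visibility trace from that character's camera along a random direction within a spread cone, applying damage with a bonus for "Head" bone hits and spawning a metal impact emitter.
; PlayFX handles fire sound and muzzle flash; Reload only plays audio.
; Persistent trace drawing and bone-name printing remain as debug output.
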(fn ConstructionScript
  (|CallParentFunction))

(fn PlayFX
  (Audio|PlaySound2D "/Game/MilitaryWeapDark/Sound/Pistol/PistolB_Fire_Cue.PistolB_Fire_Cue" 1.0 1.0 0.0 0 0)
  (Components|Activation|Activate (Variables|Default|GetFlashFX) true))

(fn LineTrace
  (bind (_cam_transform_location _returnvalue) (CallFunction|GetLInetraceParams))
  (bind _weapon_damage (Variables|Default|GetWeapon%20Damage))
  (bind _outhit (Collision|LineTraceByChannel _cam_transform_location _returnvalue "TraceTypeQuery1" false (Utilities|Array|MakeArray (Variables|Default|GetLeon%20Ref)) "Persistent"))
  (Utilities|FlowControl|Sequence
    (:then_0
      (Game|Damage|ApplyDamage (.HitActor (Collision|BreakHitResult _outhit)) (Math|Float|SelectFloat (* _weapon_damage 1.5) _weapon_damage (== (.HitBoneName (Collision|BreakHitResult _outhit)) "Head")) 0 0)
      (Development|PrintString (Utilities|String|ToString(Name) (.HitBoneName (Collision|BreakHitResult _outhit)))))
    (:then_1
      (Effects|SpawnEmitteratLocation "/Game/MilitaryWeapDark/FX/P_Impact_Metal_Medium_01.P_Impact_Metal_Medium_01" (.ImpactPoint (Collision|BreakHitResult _outhit)) (Math|Rotator|MakeRotfromX (.ImpactNormal (Collision|BreakHitResult _outhit)))))))

(fn GetLInetraceParams
  (bind _leon_ref (Variables|Default|GetLeon%20Ref))
  (bind _cam_transform (Default|GetCamTransform _leon_ref))
  (return (.location _cam_transform) (+ (.location _cam_transform) (* (Math|Random|RandomUnitVectorinConeinDegrees (Math|Vector|GetForwardVector (.rotation _cam_transform)) (Variables|Default|GetCone%20Half%20Angle%20in%20Degrees)) 1e+03))))

(fn Reload
  (Audio|PlaySound2D "/Game/MilitaryWeapDark/Sound/Pistol/Wavs/Pistol_Reload03.Pistol_Reload03" 1.0 1.0 0.0 0 0))