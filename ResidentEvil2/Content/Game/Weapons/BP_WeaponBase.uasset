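; BP_WeaponBase is a base weapon Blueprint that defines shooting, reloading and crosshair handling, and caches the player's BP_Leon character on BeginPlay.
; Shoot calls LineTrace then PlayFX, but both are empty here, as is Reload apart from a disconnected ammo assignment.
; Crosshair functions add or remove an existing widget from the viewport and resize it by scaling spread percent to a maximum pixel spread.
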(event EventBeginPlay
  (bind _asbp_leon (Utilities|Casting|CastToBP_Leon (Game|GetPlayerCharacter 0)))
  (Variables|Default|SetLeon%20Ref _asbp_leon))

(fn ConstructionScript)

(fn Shoot
  (CallFunction|LineTrace)
  (CallFunction|PlayFX))

(fn LineTrace)

(fn PlayFX)

(fn Reload)

(fn ShowCrosshair
  (params (show :type Boolean))
  (bind _crosshair (Variables|Default|GetCrosshair))
  (Utilities|IsValid (Variables|Default|GetCrosshair)
    (:Is%20Valid
      (if show
        (UserInterface|Viewport|AddtoViewport _crosshair 0)
        (else
          (Widget|RemovefromParent _crosshair))))))

(fn UpdateCrosshairSize
  (params (Spread%20Percent :type Float%20%28double-precision%29))
  (bind _output_get (Variables|Default|SetCurrent%20Spread%20Percent Spread%20Percent))
  (Default|UpdateCrosshairSize (Variables|Default|GetCrosshair) (* _output_get (Variables|Default|GetMax%20Spread%20PIxels))))